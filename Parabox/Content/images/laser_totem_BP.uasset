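; Laser totem actor for a puzzle where beams are aimed at a Globe_BP, with a reveal event that makes it visible and blocking.
; While Looking, mouse axes rotate the camera and copy its rotation to a scene component.
; Disconnected logic holds the scope view, trace-scaled laser and count of on-target totems that drives globe glow and triggers the win above two.
; Tick and startsee are empty, so that logic never runs.
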(event `showpodium`
  (bind _laser_totem (`self.laser_totem`))
  (`SceneComponent.SetVisibility` _laser_totem true false)
  (`PrimitiveComponent.SetCollisionResponseToAllChannels` _laser_totem "ECR_Block"))

(event `InputAxis|Turn Right / Left Mouse` :consume false
  (params (AxisValue :type "Float (single-precision)"))
  (if (`self.looking`)
    (`SceneComponent.K2_AddRelativeRotation` (`self.Camera`) (`KismetMathLibrary.MakeRotator` 0.0 (* (stale `InputAxis|Look Up / Down Mouse` AxisValue) -0.3) (* AxisValue 0.3)) false false :!label _label)
    (`SceneComponent.K2_SetRelativeRotation` (`self.Scene`) (`SceneComponent.RelativeRotation` (`self.Camera`)) false false)))

(event `InputAxis|Look Up / Down Mouse` :consume false
  (params (AxisValue :type "Float (single-precision)"))
  (if (`self.looking`)
    (goto _label)))

(event `self.ReceiveTick`
  (params (DeltaSeconds :type "Float (single-precision)")))

(event `startsee`)

(event `Key|E` :consume false
  (params (Key :type "Key Structure")))

(fn `UserConstructionScript`)