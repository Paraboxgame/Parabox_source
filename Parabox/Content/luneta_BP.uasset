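; Luneta is a usable scope actor that the player looks through, turning its camera with the mouse and zooming through a wheel-driven FOV timeline.
; startsee hides the pawn and shows a Scope widget; for tags one, two or three it first unhides a Lock once.
; Tick displays floored yaw and pitch, clicking when either changes.
; E restores the pawn's view and input, clearing its Zajety flag after a delay.
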(event `InputAxis|Turn Right / Left Mouse` :consume false
  (params (AxisValue :type "Float (single-precision)"))
  (if (`self.looking`)
    (`SceneComponent.K2_AddRelativeRotation` (`self.Camera`) (`KismetMathLibrary.MakeRotator` 0.0 (* (stale `InputAxis|Look Up / Down Mouse` AxisValue) -0.3) (* AxisValue 0.3)) false false :!label _label)))

(event `InputAxis|Look Up / Down Mouse` :consume false
  (params (AxisValue :type "Float (single-precision)"))
  (if (`self.looking`)
    (goto _label)))

(event `startsee`
  (if (`self.ActorHasTag` "one")
    (`|ExecutionSequence`
      (:`then_0`
        (`/Engine/EditorBlueprintResources/StandardMacros.DoOnce` false
          (:`Completed`
            (bind _returnvalue (`GameplayStatics.GetActorOfClass` "/Game/images/lock.lock_C"))
            (`/Game/images/lock.unhidelock` _returnvalue))))
      (:`then_1`
        (set `self.looking` true :!label _label_2)
        (bind _returnvalue_2 (`|CreateWidget` "/Game/scope.scope_C"))
        (`UserWidget.AddToViewport` _returnvalue_2 0)
        (`self.SetActorHiddenInGame` (`GameplayStatics.GetPlayerPawn` 0) true)))
    (elif (`self.ActorHasTag` "two")
      (`|ExecutionSequence`
        (:`then_0`
          (`/Engine/EditorBlueprintResources/StandardMacros.DoOnce` false
            (:`Completed`
              (bind _returnvalue_3 (`GameplayStatics.GetActorOfClass` "/Game/images/lock.lock_C"))
              (`/Game/images/lock.unhidelock` _returnvalue_3))))
        (:`then_1`
          (goto _label_2)))
      (elif (`self.ActorHasTag` "three")
        (`|ExecutionSequence`
          (:`then_0`
            (`/Engine/EditorBlueprintResources/StandardMacros.DoOnce` false
              (:`Completed`
                (bind _returnvalue_4 (`GameplayStatics.GetActorOfClass` "/Game/images/lock.lock_C"))
                (`/Game/images/lock.unhidelock` _returnvalue_4))))
          (:`then_1`
            (goto _label_2)))))))

(event `self.ReceiveTick`
  (params (DeltaSeconds :type "Float (single-precision)"))
  (bind (_returnvalue_roll _returnvalue_pitch _returnvalue_yaw) (`KismetMathLibrary.BreakRotator` (`PlayerCameraManager.GetCameraRotation` (`GameplayStatics.GetPlayerCameraManager` 0))))
  (bind _returnvalue (`KismetMathLibrary.FFloor` _returnvalue_pitch))
  (bind _returnvalue_2 (`KismetMathLibrary.FFloor` _returnvalue_yaw))
  (if (`self.looking`)
    (`/Engine/EditorBlueprintResources/StandardMacros.IsValid` (stale `startsee` _returnvalue_2)
      (:`Is Valid`
        (`TextBlock.SetText` (`/Game/scope.nax` (stale `startsee` _returnvalue_2)) (`KismetTextLibrary.Conv_IntToText` _returnvalue_2))
        (`TextBlock.SetText` (`/Game/scope.nay` (stale `startsee` _returnvalue_2)) (`KismetTextLibrary.Conv_IntToText` _returnvalue))
        (if (or (!= (`self.xnow`) _returnvalue_2) (!= (`self.ynow`) _returnvalue))
          (`GameplayStatics.PlaySound2D` "/Game/522319__filmmakersmanual__scope-click-sniper-rifle-4.522319__filmmakersmanual__scope-click-sniper-rifle-4" 1.0 1.0 0.0 null null))
        (set `self.xnow` _returnvalue_2)
        (set `self.ynow` _returnvalue)))))

(event `Key|E` :consume false
  (params (Key :type "Key Structure"))
  (bind _returnvalue (`GameplayStatics.GetPlayerController` 0))
  (:`Pressed`
    (if (`self.looking`)
      (`PlayerController.SetViewTargetWithBlend` (`GameplayStatics.GetPlayerController` 0) (`GameplayStatics.GetPlayerPawn` 0) 0.0 "VTBlend_Linear" 0.0 false)
      (set `self.looking` false)
      (`/Engine/EditorBlueprintResources/StandardMacros.IsValid` (stale `startsee` _returnvalue_2)
        (:`Is Valid`
          (`Widget.RemoveFromParent` (stale `startsee` _returnvalue_2)))
        (:`Is Not Valid`
          _))
      (`Controller.SetIgnoreMoveInput` _returnvalue false)
      (`Controller.SetIgnoreLookInput` _returnvalue false)
      (bind _asbp_third_person_character_zombie (cast `` (`GameplayStatics.GetPlayerPawn` 0)))
      (`|ExecutionSequence`
        (:`then_0`
          (`KismetSystemLibrary.Delay` 1.0)
          (set `/Game/luneta_BP.zajety` false _asbp_third_person_character_zombie))
        (:`then_1`
          (`self.SetActorHiddenInGame` (`GameplayStatics.GetPlayerPawn` 0) false))))))

(event `InputAxisKey|MouseWheelAxis` :consume false
  (params (AxisValue :type "Float (single-precision)"))
  (if (> AxisValue 0.0)
    (bind (_direction _newtrack_0) (`Timeline|Timeline_0` :!label _label_3)
      (:`Update`
        (`CameraComponent.SetFieldOfView` (`self.Camera`) _newtrack_0)))
    (elif (< AxisValue 0.0)
      (goto _label_3 :!via `Reverse`))))

(fn `UserConstructionScript`)