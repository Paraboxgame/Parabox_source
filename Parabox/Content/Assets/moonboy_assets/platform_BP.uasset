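; Scrolling platform for a vertical jumper that moves along Z each Tick at the Speed read from Moonb_char, simulating the player's climb.
; Once below a lower Z limit, it recycles to a random Y and height near the top and destroys its previous pickup.
; It then makes cascading low-chance rolls to spawn a Rocket, Boots or Jetpack at its Scene component, attaching it and storing it in Act.
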(event `self.ReceiveTick`
  (params (DeltaSeconds :type "Float (single-precision)"))
  (bind (_returnvalue_x _returnvalue_y _returnvalue_z) (`KismetMathLibrary.BreakVector` (`self.K2_GetActorLocation`)))
  (bind _act (`self.act`))
  (bind _returnvalue (`GameplayStatics.GetActorOfClass` "/Game/Assets/moonboy_assets/moonb_char.moonb_char_C"))
  (`self.K2_AddActorWorldOffset` (`KismetMathLibrary.MakeVector` 0.0 0.0 (* (`/Game/Assets/moonboy_assets/moonb_char.speed` _returnvalue) DeltaSeconds)))
  (if (< _returnvalue_z -400.0)
    (`self.K2_SetActorLocation` (`KismetMathLibrary.MakeVector` 0.0 (`KismetMathLibrary.RandomFloatInRange` -260.0 260.0) (`KismetMathLibrary.RandomFloatInRange` 400.0 450.0)))
    (`/Engine/EditorBlueprintResources/StandardMacros.IsValid` _act
      (:`Is Valid`
        (`self.K2_DestroyActor` _act))
      (:`Is Not Valid`
        _))
    (if (> (`KismetMathLibrary.RandomIntegerInRange` 0 20) 18)
      (bind _returnvalue_2 (`|SpawnActorFromClass` "/Game/Assets/moonboy_assets/rocket.rocket_C" (`KismetMathLibrary.MakeTransform` (`SceneComponent.K2_GetComponentLocation` (`self.Scene`)) (struct :`Yaw` 180.0)) "Undefined" "OverrideRootScale" null 0.0 null))
      (set `self.act` _returnvalue_2)
      (`self.K2_AttachToActor` _returnvalue_2 self "scene" "SnapToTarget" "KeepRelative" "KeepRelative" true)
      (elif (> (`KismetMathLibrary.RandomIntegerInRange` 0 20) 18)
        (bind _returnvalue_3 (`|SpawnActorFromClass` "/Game/Assets/moonboy_assets/boots.boots_C" (`KismetMathLibrary.MakeTransform` (`SceneComponent.K2_GetComponentLocation` (`self.Scene`)) (struct :`Yaw` 180.0)) "Undefined" "OverrideRootScale" null 0.0 null))
        (set `self.act` _returnvalue_3)
        (`self.K2_AttachToActor` _returnvalue_3 self "scene" "SnapToTarget" "KeepRelative" "KeepRelative" true)
        (elif (> (`KismetMathLibrary.RandomIntegerInRange` 0 20) 18)
          (bind _returnvalue_4 (`|SpawnActorFromClass` "/Game/Assets/moonboy_assets/jetpack.jetpack_C" (`KismetMathLibrary.MakeTransform` (`SceneComponent.K2_GetComponentLocation` (`self.Scene`)) (struct :`Yaw` 180.0)) "Undefined" "OverrideRootScale" null 0.0 null))
          (set `self.act` _returnvalue_4)
          (`self.K2_AttachToActor` _returnvalue_4 self "scene" "SnapToTarget" "KeepRelative" "KeepRelative" true))))))

(fn `UserConstructionScript`)