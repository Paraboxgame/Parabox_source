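; Moving platform that scrolls vertically while sliding side to side along Y.
; Each Tick, it looks up the Moonb_char actor and offsets Z by that character's Speed, scaled by delta time.
; Dropping below a lower limit recycles it to a random Y and height near the top.
; Sideways motion adds MOVE per frame, unscaled by delta time, and flips its sign beyond the Y bounds.
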(event `self.ReceiveTick`
  (params (DeltaSeconds :type "Float (single-precision)"))
  (bind (_returnvalue_x _returnvalue_y) (`KismetMathLibrary.BreakVector` (`self.K2_GetActorLocation`)))
  (bind (_returnvalue_x_2 _returnvalue_y_2 _returnvalue_z) (`KismetMathLibrary.BreakVector` (`self.K2_GetActorLocation`)))
  (`|ExecutionSequence`
    (:`then_0`
      (bind _returnvalue (`GameplayStatics.GetActorOfClass` "/Game/Assets/moonboy_assets/moonb_char.moonb_char_C"))
      (`self.K2_AddActorWorldOffset` (`KismetMathLibrary.MakeVector` 0.0 0.0 (* (`/Game/Assets/moonboy_assets/moonb_char.speed` _returnvalue) DeltaSeconds)))
      (if (< _returnvalue_z -400.0)
        (`self.K2_SetActorLocation` (`KismetMathLibrary.MakeVector` 0.0 (`KismetMathLibrary.RandomFloatInRange` -260.0 260.0) (`KismetMathLibrary.RandomFloatInRange` 400.0 450.0)))))
    (:`then_1`
      (`self.K2_AddActorWorldOffset` (`KismetMathLibrary.MakeVector` 0.0 (`self.MOVE`)))
      (if (or (> _returnvalue_y 260.0) (< _returnvalue_y -260.0))
        (set `self.MOVE` (* (`self.MOVE`) -1.0))))))

(fn `UserConstructionScript`)