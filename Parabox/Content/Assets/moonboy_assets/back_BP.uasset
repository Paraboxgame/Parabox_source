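; Background actor Blueprint that drives the speed of the Moonboy background material from the player character.
; On BeginPlay it finds the Moonb_char actor and creates a dynamic instance of the background material on its Plane.
; Each Tick it sets the material's speed parameter to the character's Dist divided by a constant, alongside a leftover debug print.
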(event `self.ReceiveBeginPlay`
  (bind _returnvalue (`GameplayStatics.GetActorOfClass` "/Game/Assets/moonboy_assets/moonb_char.moonb_char_C"))
  (set `self.NewVar_0` _returnvalue)
  (bind _returnvalue_2 (`PrimitiveComponent.CreateDynamicMaterialInstance` (`self.Plane`) 0 "/Game/Assets/moonboy_assets/Moonboy_background_Mat_Inst.Moonboy_background_Mat_Inst" "None"))
  (set `self.NewVar_1` _returnvalue_2))

(event `self.ReceiveTick`
  (params (DeltaSeconds :type "Float (single-precision)"))
  (`MaterialInstanceDynamic.SetScalarParameterValue` (`self.NewVar_1`) "speed" (/ (`/Game/Assets/moonboy_assets/moonb_char.dist` (`self.NewVar_0`)) 500.0))
  (`KismetSystemLibrary.PrintString` "Hello" true true (struct :`G` 0.66 :`B` 1.0 :`A` 1.0) 0.0))

(fn `UserConstructionScript`)