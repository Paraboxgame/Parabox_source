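; BOAT_bp is a boat actor meant to be steered by where the player pawn stands.
; While Move is set, Tick yaws it toward whichever of Rig or Lef is set alone and drives ProjectileMovement along its forward vector, otherwise zeroing velocity when Move is off.
; The Box, Left and Right overlap events are empty, and the player-check logic that would set those flags is disconnected, so this graph never changes them.
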(event `self.ReceiveTick`
  (params (DeltaSeconds :type "Float (single-precision)"))
  (bind _projectilemovement (`self.ProjectileMovement`))
  (bind _returnvalue (* (`self.GetActorForwardVector`) 200))
  (if (`self.move`)
    (if (and (`self.rig`) (not (`self.lef`)))
      (`self.K2_AddActorWorldRotation` (struct :`Yaw` 0.2))
      (set `MovementComponent.Velocity` _returnvalue _projectilemovement)
      (elif (and (`self.lef`) (not (`self.rig`)))
        (`self.K2_AddActorWorldRotation` (struct :`Yaw` -0.2))
        (set `MovementComponent.Velocity` _returnvalue _projectilemovement)))
    (else
      (set `MovementComponent.Velocity` (0.0 0.0 0.0) _projectilemovement))))

(event `self.Box.OnComponentBeginOverlap`
  (params (OverlappedComponent :type "PrimitiveComponent Object Reference") (OtherActor :type "Actor Object Reference") (OtherComp :type "PrimitiveComponent Object Reference") (OtherBodyIndex :type Integer) (bFromSweep :type Boolean) (SweepResult :type "HitResult Structure (by ref)")))

(event `self.Box.OnComponentEndOverlap`
  (params (OverlappedComponent :type "PrimitiveComponent Object Reference") (OtherActor :type "Actor Object Reference") (OtherComp :type "PrimitiveComponent Object Reference") (OtherBodyIndex :type Integer)))

(event `self.left.OnComponentBeginOverlap`
  (params (OverlappedComponent :type "PrimitiveComponent Object Reference") (OtherActor :type "Actor Object Reference") (OtherComp :type "PrimitiveComponent Object Reference") (OtherBodyIndex :type Integer) (bFromSweep :type Boolean) (SweepResult :type "HitResult Structure (by ref)")))

(event `self.left.OnComponentEndOverlap`
  (params (OverlappedComponent :type "PrimitiveComponent Object Reference") (OtherActor :type "Actor Object Reference") (OtherComp :type "PrimitiveComponent Object Reference") (OtherBodyIndex :type Integer)))

(event `self.right.OnComponentBeginOverlap`
  (params (OverlappedComponent :type "PrimitiveComponent Object Reference") (OtherActor :type "Actor Object Reference") (OtherComp :type "PrimitiveComponent Object Reference") (OtherBodyIndex :type Integer) (bFromSweep :type Boolean) (SweepResult :type "HitResult Structure (by ref)")))

(event `self.right.OnComponentEndOverlap`
  (params (OverlappedComponent :type "PrimitiveComponent Object Reference") (OtherActor :type "Actor Object Reference") (OtherComp :type "PrimitiveComponent Object Reference") (OtherBodyIndex :type Integer)))

(fn `UserConstructionScript`)