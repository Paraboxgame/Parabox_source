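; Wall actor that displays six NFT images on its plane components.
; On BeginPlay, each plane takes the next texture from the NFT_images actor's array and advances that actor's shared Num counter, so successive walls continue through the list.
; Each texture is cached locally and applied through a dynamic material instance of Nft_mat_instance.
; The counter has no bounds check or wraparound.
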(event `self.ReceiveBeginPlay`
  (`|ExecutionSequence`
    (:`then_0`
      (bind _returnvalue (`GameplayStatics.GetActorOfClass` "/Game/Assets/nftimages/NFT_images.NFT_images_C"))
      (bind _num (`/Game/Assets/nftimages/NFT_images.num` _returnvalue))
      (`KismetArrayLibrary.Array_Add` (`self.nfts`) (`|GetArrayItem` (`/Game/Assets/nftimages/NFT_images.nfts` _returnvalue) _num))
      (set `/Game/Assets/nftimages/NFT_images.num` (+ _num 1) _returnvalue)
      (bind _returnvalue_2 (`PrimitiveComponent.CreateDynamicMaterialInstance` (`self.Plane2`) 0 "/Game/Assets/nftimages/nft_mat_instance.nft_mat_instance" "None"))
      (`MaterialInstanceDynamic.SetTextureParameterValue` _returnvalue_2 "param" (`|GetArrayItem` (`self.nfts`))))
    (:`then_1`
      (bind _returnvalue_3 (`GameplayStatics.GetActorOfClass` "/Game/Assets/nftimages/NFT_images.NFT_images_C"))
      (bind _num_2 (`/Game/Assets/nftimages/NFT_images.num` _returnvalue_3))
      (`KismetArrayLibrary.Array_Add` (`self.nfts`) (`|GetArrayItem` (`/Game/Assets/nftimages/NFT_images.nfts` _returnvalue_3) _num_2))
      (set `/Game/Assets/nftimages/NFT_images.num` (+ _num_2 1) _returnvalue_3)
      (bind _returnvalue_4 (`PrimitiveComponent.CreateDynamicMaterialInstance` (`self.Plane1`) 0 "/Game/Assets/nftimages/nft_mat_instance.nft_mat_instance" "None"))
      (`MaterialInstanceDynamic.SetTextureParameterValue` _returnvalue_4 "param" (`|GetArrayItem` (`self.nfts`) 1)))
    (:`then_2`
      (bind _returnvalue_5 (`GameplayStatics.GetActorOfClass` "/Game/Assets/nftimages/NFT_images.NFT_images_C"))
      (bind _num_3 (`/Game/Assets/nftimages/NFT_images.num` _returnvalue_5))
      (`KismetArrayLibrary.Array_Add` (`self.nfts`) (`|GetArrayItem` (`/Game/Assets/nftimages/NFT_images.nfts` _returnvalue_5) _num_3))
      (set `/Game/Assets/nftimages/NFT_images.num` (+ _num_3 1) _returnvalue_5)
      (bind _returnvalue_6 (`PrimitiveComponent.CreateDynamicMaterialInstance` (`self.Plane`) 0 "/Game/Assets/nftimages/nft_mat_instance.nft_mat_instance" "None"))
      (`MaterialInstanceDynamic.SetTextureParameterValue` _returnvalue_6 "param" (`|GetArrayItem` (`self.nfts`) 2)))
    (:`then_3`
      (bind _returnvalue_7 (`GameplayStatics.GetActorOfClass` "/Game/Assets/nftimages/NFT_images.NFT_images_C"))
      (bind _num_4 (`/Game/Assets/nftimages/NFT_images.num` _returnvalue_7))
      (`KismetArrayLibrary.Array_Add` (`self.nfts`) (`|GetArrayItem` (`/Game/Assets/nftimages/NFT_images.nfts` _returnvalue_7) _num_4))
      (set `/Game/Assets/nftimages/NFT_images.num` (+ _num_4 1) _returnvalue_7)
      (bind _returnvalue_8 (`PrimitiveComponent.CreateDynamicMaterialInstance` (`self.Plane3`) 0 "/Game/Assets/nftimages/nft_mat_instance.nft_mat_instance" "None"))
      (`MaterialInstanceDynamic.SetTextureParameterValue` _returnvalue_8 "param" (`|GetArrayItem` (`self.nfts`) 3)))
    (:`then_4`
      (bind _returnvalue_9 (`GameplayStatics.GetActorOfClass` "/Game/Assets/nftimages/NFT_images.NFT_images_C"))
      (bind _num_5 (`/Game/Assets/nftimages/NFT_images.num` _returnvalue_9))
      (`KismetArrayLibrary.Array_Add` (`self.nfts`) (`|GetArrayItem` (`/Game/Assets/nftimages/NFT_images.nfts` _returnvalue_9) _num_5))
      (set `/Game/Assets/nftimages/NFT_images.num` (+ _num_5 1) _returnvalue_9)
      (bind _returnvalue_10 (`PrimitiveComponent.CreateDynamicMaterialInstance` (`self.Plane4`) 0 "/Game/Assets/nftimages/nft_mat_instance.nft_mat_instance" "None"))
      (`MaterialInstanceDynamic.SetTextureParameterValue` _returnvalue_10 "param" (`|GetArrayItem` (`self.nfts`) 4)))
    (:`then_5`
      (bind _returnvalue_11 (`GameplayStatics.GetActorOfClass` "/Game/Assets/nftimages/NFT_images.NFT_images_C"))
      (bind _num_6 (`/Game/Assets/nftimages/NFT_images.num` _returnvalue_11))
      (`KismetArrayLibrary.Array_Add` (`self.nfts`) (`|GetArrayItem` (`/Game/Assets/nftimages/NFT_images.nfts` _returnvalue_11) _num_6))
      (set `/Game/Assets/nftimages/NFT_images.num` (+ _num_6 1) _returnvalue_11)
      (bind _returnvalue_12 (`PrimitiveComponent.CreateDynamicMaterialInstance` (`self.Plane5`) 0 "/Game/Assets/nftimages/nft_mat_instance.nft_mat_instance" "None"))
      (`MaterialInstanceDynamic.SetTextureParameterValue` _returnvalue_12 "param" (`|GetArrayItem` (`self.nfts`) 5)))))

(fn `UserConstructionScript`)