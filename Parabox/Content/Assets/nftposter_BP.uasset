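; Poster actor that displays one texture from a shared NFT image collection on its plane mesh.
; On BeginPlay it finds the NFT_images actor, copies the texture at that actor's Num index and increments the counter, so successive posters draw successive images.
; It then creates a dynamic material instance on Plane1 and applies the copied texture as a parameter.
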(event `self.ReceiveBeginPlay`
  (bind _returnvalue (`GameplayStatics.GetActorOfClass` "/Game/Assets/nftimages/NFT_images.NFT_images_C"))
  (bind _num (`/Game/Assets/nftimages/NFT_images.num` _returnvalue))
  (`KismetArrayLibrary.Array_Add` (`self.nfts`) (`|GetArrayItem` (`/Game/Assets/nftimages/NFT_images.nfts` _returnvalue) _num))
  (set `/Game/Assets/nftimages/NFT_images.num` (+ _num 1) _returnvalue)
  (bind _returnvalue_2 (`PrimitiveComponent.CreateDynamicMaterialInstance` (`self.Plane1`) 0 "/Game/Assets/nftimages/nft_mat_instance.nft_mat_instance" "None"))
  (`MaterialInstanceDynamic.SetTextureParameterValue` _returnvalue_2 "param" (`|GetArrayItem` (`self.nfts`))))

(fn `UserConstructionScript`)