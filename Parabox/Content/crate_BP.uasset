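; Treasure crate Blueprint with lasers that can be taken and an animated opening, both run by custom events.
; The takelasers event hides the crate's three laser components, calls Hidelock on the Lock actor and calls Showpodium on every Laser_totem_BP.
; The opentreasure event plays a gate sound while a timeline rolls a scene component, then sets Opened when finished.
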(event `takelasers`
  (`SceneComponent.SetVisibility` (`self.laser-1`) false false)
  (`SceneComponent.SetVisibility` (`self.laser-2`) false false)
  (`SceneComponent.SetVisibility` (`self.laser-0`) false false)
  (bind _returnvalue (`GameplayStatics.GetActorOfClass` "/Game/images/lock.lock_C"))
  (`/Game/images/lock.hidelock` _returnvalue)
  (bind _outactors (`GameplayStatics.GetAllActorsOfClass` "/Game/images/laser_totem_BP.laser_totem_BP_C"))
  (for _array_element _outactors
    (`/Game/images/laser_totem_BP.showpodium` _array_element)))

(event `opentreasure`
  (`GameplayStatics.PlaySound2D` "/Game/96173__robinhood76__01657-opening-small-gate.96173__robinhood76__01657-opening-small-gate" 1.0 1.0 0.0 null null)
  (bind (_direction _newtrack_0) (`Timeline|Timeline_0` :!via `PlayFromStart`)
    (:`Update`
      (`SceneComponent.K2_SetRelativeRotation` (`self.Scene`) (`KismetMathLibrary.MakeRotator` _newtrack_0) false false))
    (:`Finished`
      (set `self.opened` true))))

(fn `UserConstructionScript`)