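; Chess board actor that tracks white and black players and the current turn, and spawns a camera for each side at start.
; Reset clears both players through a server/multicast-named event chain, then replaces the actor with a fresh copy at the same transform.
; Helpers strip move-square actors and custom-depth highlights from board children, resetting piece materials through the Chess_pawn interface.
; Pawn-move and board-reset chains end in empty events.
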(event `destroy_multi`
  (params (NewParam :type "/Game/chess_game_BP Object Reference") (NewParam2 :type "Transform Structure"))
  (bind _player_whites (`self.player_whites`))
  (bind _player_blacks (`self.player_blacks`))
  (`/Engine/EditorBlueprintResources/StandardMacros.IsValid` _player_whites
    (:`Is Valid`
      (`/Game/Assets/ThirdPerson/Blueprints/BP_ThirdPersonCharacter.exitchessserv` _player_whites)
      (set `self.player_whites` null))
    (:`Is Not Valid`
      _))
  (`/Engine/EditorBlueprintResources/StandardMacros.IsValid` _player_blacks
    (:`Is Valid`
      (`/Game/Assets/ThirdPerson/Blueprints/BP_ThirdPersonCharacter.exitchessserv` _player_blacks))
    (:`Is Not Valid`
      _))
  (set `self.player_blacks` null))

(event `destroy_serv`
  (params (NewParam :type "/Game/chess_game_BP Object Reference") (NewParam2 :type "Transform Structure"))
  (`self.destroy_multi` null)
  (`|SpawnActorFromClass` "chess_game_BP_C" NewParam2 "AlwaysSpawn" "OverrideRootScale" null null)
  (`self.K2_DestroyActor` self))

(event `destroyme`
  (params (NewParam :type "/Game/chess_game_BP Object Reference") (NewParam2 :type "Transform Structure"))
  (`self.destroy_serv` null (`self.GetTransform`)))

(event `movepawn`
  (params (who :type "Actor Object Reference") (where :type "Vector Structure")))

(event `movepawnserver`
  (params (where :type "Vector Structure") (who :type "Actor Object Reference"))
  (`self.movepawnmulti` (stale `movepawn` where) (stale `movepawn` who)))

(event `movepawnmulti`
  (params (where :type "Vector Structure") (who :type "Actor Object Reference")))

(event `nextturn`
  (if (`self.whitemove`)
    (set `self.whitemove` false)
    (else
      (set `self.whitemove` true))))

(event `resetserver`
  (`self.resetmulti`))

(event `resetboard`
  (`self.resetserver`))

(event `resetmulti`)

(event `rempola`
  (`self.rempolaserv`))

(event `rempolaserv`
  (`self.rempola_multi`))

(event `rempola_multi`
  (for _array_element (`SceneComponent.GetChildrenComponents` (`self.chessboard_model`) true)
    (`/Engine/EditorBlueprintResources/StandardMacros.IsValid` _array_element
      (:`Is Valid`
        (bind _aschild_actor_component (cast `ChildActorComponent` _array_element))
        (bind _aspole_ruch (cast `/Game/pole_ruch` (`ChildActorComponent.ChildActor` _aschild_actor_component)))
        (`/Engine/EditorBlueprintResources/StandardMacros.IsValid` _aspole_ruch
          (:`Is Valid`
            (`self.K2_DestroyActor` _aspole_ruch)))))))

(event `renderoff`
  (for _array_element (`SceneComponent.GetChildrenComponents` (`self.chessboard_model`) true)
    (bind _asstatic_mesh_component (cast `StaticMeshComponent` _array_element))
    (`PrimitiveComponent.SetRenderCustomDepth` _asstatic_mesh_component false)
    (bind _returnvalue (`ActorComponent.GetOwner` _asstatic_mesh_component))
    (if (`KismetSystemLibrary.DoesImplementInterface` _returnvalue "/Game/chess_pawn.chess_pawn_C")
      (message `/Game/chess_pawn.resetmat` _returnvalue)))
  (`self.rempola`))

(event `self.ReceiveTick`
  (params (DeltaSeconds :type "Float (single-precision)")))

(event `showlogserv`
  (`KismetSystemLibrary.PrintString` (`KismetStringLibrary.Concat_StrStr` (`KismetStringLibrary.Conv_BoolToString` (`self.whitemove`)) "-" (`KismetStringLibrary.Conv_BoolToString` (`self.whites`)) "-" (`KismetStringLibrary.Conv_BoolToString` (`self.blacks`)) "-whiteplayer-" (`KismetSystemLibrary.GetDisplayName` (`self.player_whites`)) "-blackplayer-" (`KismetSystemLibrary.GetDisplayName` (`self.player_blacks`))) true true (struct :`G` 0.66 :`B` 1.0 :`A` 1.0) 0.0))

(event `self.ReceiveBeginPlay`
  (bind _cam1 (`self.cam1`))
  (bind _cam2 (`self.cam2`))
  (bind _returnvalue (`|SpawnActorFromClass` "/Script/Engine.CameraActor" (`KismetMathLibrary.MakeTransform` (`SceneComponent.K2_GetComponentLocation` _cam1) (`SceneComponent.K2_GetComponentRotation` _cam1)) "Undefined" "OverrideRootScale" null null))
  (set `self.cam_w` _returnvalue)
  (bind _returnvalue_2 (`|SpawnActorFromClass` "/Script/Engine.CameraActor" (`KismetMathLibrary.MakeTransform` (`SceneComponent.K2_GetComponentLocation` _cam2) (`SceneComponent.K2_GetComponentRotation` _cam2)) "Undefined" "OverrideRootScale" null null))
  (set `self.cam_B` _returnvalue_2))

(event `checkreset`
  (`KismetSystemLibrary.PrintString` "reseting" :!label _label)
  (set `self.whitemove` true)
  (set `self.whites` false)
  (set `self.blacks` false)
  (`self.destroyme` null))

(event `checkresetmulti`
  (goto _label))

(event `resettime`
  (`KismetSystemLibrary.PrintString` "start")
  (bind (_direction _newtrack_0) (`Timeline|runtime` :!via `PlayFromStart`)
    (:`Update`
      (set `self.time` (`KismetMathLibrary.FCeil` _newtrack_0)))))

(fn `UserConstructionScript`
  (for _array_element (`SceneComponent.GetChildrenComponents` (`self.chessboard_model`) true)
    (bind _asstatic_mesh_component (cast `StaticMeshComponent` _array_element))
    (`PrimitiveComponent.SetRenderCustomDepth` _asstatic_mesh_component false)))