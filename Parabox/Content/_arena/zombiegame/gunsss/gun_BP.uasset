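; Spinning gun pickup for the zombie arena that gives the player one of six random weapons.
; The construction script rolls a gun number and sets the matching mesh, and Tick rotates it.
; When the player overlaps the sphere, it sets the character's gun type and ammo, refreshes weapon and ammo, and plays a sound.
; The pickup then hides and disables itself for a random delay before reappearing with a freshly rolled gun.
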(event `reset`
  (bind _staticmesh (`self.StaticMesh`))
  (set `self.gunnum` (`KismetMathLibrary.RandomIntegerInRange` 1 6))
  (switch `int` (`self.gunnum`)
    (:`1`
      (`StaticMeshComponent.SetStaticMesh` _staticmesh "/Game/_arena/zombiegame/gunsss/gun_1_automaticpistol.gun_1_automaticpistol"))
    (:`2`
      (`StaticMeshComponent.SetStaticMesh` _staticmesh "/Game/_arena/zombiegame/gunsss/gun_2_revolver.gun_2_revolver"))
    (:`3`
      (`StaticMeshComponent.SetStaticMesh` _staticmesh "/Game/_arena/zombiegame/gunsss/gun_3_riffle.gun_3_riffle"))
    (:`4`
      (`StaticMeshComponent.SetStaticMesh` _staticmesh "/Game/_arena/zombiegame/gunsss/gun_4_crossbow.gun_4_crossbow"))
    (:`5`
      (`StaticMeshComponent.SetStaticMesh` _staticmesh "/Game/_arena/zombiegame/gunsss/gun_5_shotgun.gun_5_shotgun"))
    (:`6`
      (`StaticMeshComponent.SetStaticMesh` _staticmesh "/Game/_arena/zombiegame/gunsss/gun_6_ak.gun_6_ak"))))

(event `self.ReceiveTick`
  (params (DeltaSeconds :type "Float (single-precision)"))
  (`SceneComponent.K2_AddLocalRotation` (`self.Scene`) (struct :`Yaw` 1.0) false false))

(event `self.Sphere.OnComponentBeginOverlap`
  (params (OverlappedComponent :type "PrimitiveComponent Object Reference") (OtherActor :type "Actor Object Reference") (OtherComp :type "PrimitiveComponent Object Reference") (OtherBodyIndex :type Integer) (bFromSweep :type Boolean) (SweepResult :type "HitResult Structure (by ref)"))
  (bind _returnvalue (`GameplayStatics.GetPlayerPawn` 0))
  (bind _gunnum (`self.gunnum`))
  (bind _staticmesh (`self.StaticMesh`))
  (if (`self.off`)
    _
    (elif (== OtherActor _returnvalue)
      (`GameplayStatics.PlaySound2D` "/Game/_arena/zombiegame/gunsss/new_gun.new_gun" 1.0 1.0 0.0 null null)
      (bind _asbp_third_person_character_zombie (cast `/Game/Assets/ThirdPerson/Blueprints/BP_ThirdPersonCharacter_zombies` _returnvalue))
      (`|ExecutionSequence`
        (:`then_0`
          (set `/Game/Assets/ThirdPerson/Blueprints/BP_ThirdPersonCharacter_zombies.guntype` _gunnum _asbp_third_person_character_zombie)
          (switch `int` _gunnum
            (:`1`
              (set `/Game/Assets/ThirdPerson/Blueprints/BP_ThirdPersonCharacter_zombies.ammo` 30 _asbp_third_person_character_zombie))
            (:`2`
              (set `/Game/Assets/ThirdPerson/Blueprints/BP_ThirdPersonCharacter_zombies.ammo` 10 _asbp_third_person_character_zombie))
            (:`3`
              (set `/Game/Assets/ThirdPerson/Blueprints/BP_ThirdPersonCharacter_zombies.ammo` 15 _asbp_third_person_character_zombie))
            (:`4`
              (set `/Game/Assets/ThirdPerson/Blueprints/BP_ThirdPersonCharacter_zombies.ammo` 15 _asbp_third_person_character_zombie))
            (:`5`
              (set `/Game/Assets/ThirdPerson/Blueprints/BP_ThirdPersonCharacter_zombies.ammo` 10 _asbp_third_person_character_zombie))
            (:`6`
              (set `/Game/Assets/ThirdPerson/Blueprints/BP_ThirdPersonCharacter_zombies.ammo` 100 _asbp_third_person_character_zombie))))
        (:`then_1`
          (`/Game/Assets/ThirdPerson/Blueprints/BP_ThirdPersonCharacter_zombies.newweapon` _asbp_third_person_character_zombie)
          (`/Game/Assets/ThirdPerson/Blueprints/BP_ThirdPersonCharacter_zombies.updateammo` _asbp_third_person_character_zombie)
          (`SceneComponent.SetVisibility` _staticmesh false false)
          (set `self.off` true)
          (`KismetSystemLibrary.Delay` (`KismetMathLibrary.RandomFloatInRange` 10.0 30.0))
          (set `self.off` false)
          (`SceneComponent.SetVisibility` _staticmesh true false)
          (`self.reset`))))))

(fn `UserConstructionScript`
  (bind _staticmesh (`self.StaticMesh`))
  (set `self.gunnum` (`KismetMathLibrary.RandomIntegerInRange` 1 6))
  (switch `int` (`self.gunnum`)
    (:`1`
      (`StaticMeshComponent.SetStaticMesh` _staticmesh "/Game/_arena/zombiegame/gunsss/gun_1_automaticpistol.gun_1_automaticpistol"))
    (:`2`
      (`StaticMeshComponent.SetStaticMesh` _staticmesh "/Game/_arena/zombiegame/gunsss/gun_2_revolver.gun_2_revolver"))
    (:`3`
      (`StaticMeshComponent.SetStaticMesh` _staticmesh "/Game/_arena/zombiegame/gunsss/gun_3_riffle.gun_3_riffle"))
    (:`4`
      (`StaticMeshComponent.SetStaticMesh` _staticmesh "/Game/_arena/zombiegame/gunsss/gun_4_crossbow.gun_4_crossbow"))
    (:`5`
      (`StaticMeshComponent.SetStaticMesh` _staticmesh "/Game/_arena/zombiegame/gunsss/gun_5_shotgun.gun_5_shotgun"))
    (:`6`
      (`StaticMeshComponent.SetStaticMesh` _staticmesh "/Game/_arena/zombiegame/gunsss/gun_6_ak.gun_6_ak"))))