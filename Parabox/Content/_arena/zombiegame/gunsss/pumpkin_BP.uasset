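; Pumpkin collectible for the zombie game that adds to the player character's pumpkin count when picked up.
; Sphere overlap increments the count on the player pawn, updates the zombie HUD text, plays coin and laugh sounds, then destroys the actor.
; The overlapping actor is never checked, so any overlap credits the player.
; The construction script randomizes scale per axis and yaw for visual variety.
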(event `self.Sphere.OnComponentBeginOverlap`
  (params (OverlappedComponent :type "PrimitiveComponent Object Reference") (OtherActor :type "Actor Object Reference") (OtherComp :type "PrimitiveComponent Object Reference") (OtherBodyIndex :type Integer) (bFromSweep :type Boolean) (SweepResult :type "HitResult Structure (by ref)"))
  (bind _asbp_third_person_character_zombies (cast `/Game/Assets/ThirdPerson/Blueprints/BP_ThirdPersonCharacter_zombies` (`GameplayStatics.GetPlayerPawn` 0)))
  (bind _result (`/Engine/EditorBlueprintResources/StandardMacros.IncrementInt` (`/Game/Assets/ThirdPerson/Blueprints/BP_ThirdPersonCharacter_zombies.pumpkins` _asbp_third_person_character_zombies))
    (:`  `
      (bind _foundwidgets (`WidgetBlueprintLibrary.GetAllWidgetsOfClass` "/Game/_arena/areaassets/zombiehud_zz.zombiehud_zz_C"))
      (`TextBlock.SetText` (`/Game/_arena/areaassets/zombiehud_zz.pumpkin` (`|GetArrayItem` _foundwidgets)) (`KismetTextLibrary.Conv_IntToText` _result))
      (`GameplayStatics.PlaySound2D` "/Game/_arena/zombiegame/zapsplat_multimedia_game_sound_collect_treasure_coin_003_40561.zapsplat_multimedia_game_sound_collect_treasure_coin_003_40561" 1.0 1.0 0.0 null null)
      (`GameplayStatics.PlaySound2D` "/Game/_arena/zombiegame/zapsplat_horror_laugh_male_demonic_wide_heavily_processed_005_71397.zapsplat_horror_laugh_male_demonic_wide_heavily_processed_005_71397" 1.0 1.0 0.0 null null)
      (`self.K2_DestroyActor`))))

(fn `UserConstructionScript`
  (bind _returnvalue (`KismetMathLibrary.RandomFloatInRange` 0.7 0.9))
  (bind _scene (`self.Scene`))
  (`SceneComponent.SetWorldScale3D` _scene (`KismetMathLibrary.MakeVector` _returnvalue _returnvalue _returnvalue))
  (`SceneComponent.K2_SetWorldRotation` _scene (`KismetMathLibrary.MakeRotator` 0.0 0.0 (`KismetMathLibrary.RandomFloatInRange` 0.0 360.0)) false false))